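; Game director that runs an in-game clock and activates anomalies at randomly scheduled times.
; On BeginPlay it caches all BP_Anomaly actors, schedules the first spawn and starts a looping timer that advances the minute and hour with day rollover.
; When the clock matches the scheduled time, it activates an inactive anomaly, only if it casts to BP_Door_Anomaly_Child, then schedules the next using a random delay.
; Debug prints trace time, scheduling and activation.
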(event Custom|AdvanceTime_Event
  (CallFunction|AdvanceTime)
  (CallFunction|DebugTime))

(event EventBeginPlay
  (Utilities|Time|SetTimerbyEvent (delegate Custom|AdvanceTime_Event) (Variables|Default|GetSecondsPerGameMinute) true)
  (bind _outactors (Actor|GetAllActorsOfClass "/Game/MainContent/Blueprints/System/BP_Anomaly.BP_Anomaly_C"))
  (bind _output_get (Variables|Default|SetAnomalies _outactors))
  (CallFunction|ScheduleNextAnomaly)
  (Development|PrintString (Utilities|String|ToString(Integer) (Utilities|Array|Length _output_get))))

(event Collision|EventActorBeginOverlap
  (params (OtherActor :type Actor%20Object%20Reference)))

(event EventTick
  (params (DeltaSeconds :type Float%20%28single-precision%29)))

(fn ConstructionScript)

(fn AdvanceTime
  (bind _nextspawnminute (Variables|Default|GetNextSpawnMinute))
  (bind _nextspawnhour (Variables|Default|GetNextSpawnHour))
  (Variables|Default|SetCurrentMinute (+ (Variables|Default|GetCurrentMinute) 1))
  (if (>= (Variables|Default|GetCurrentMinute) 60)
    (Variables|Default|SetCurrentMinute 0)
    (Variables|Default|SetCurrentHour (+ (Variables|Default|GetCurrentHour) 1))
    (if (>= (Variables|Default|GetCurrentHour) 24)
      (Variables|Default|SetCurrentHour 0)
      (if (Variables|Default|GetbSpawnScheduled)
        (if (and (== (Variables|Default|GetCurrentHour) (Variables|Default|GetNextSpawnHour)) (== (Variables|Default|GetCurrentMinute) (Variables|Default|GetNextSpawnMinute)))
          (bind _array_element (Utilities|Array|ForEachLoopwithBreak (Variables|Default|GetAnomalies) :!label _label)
            (:LoopBody
              (if (not (Variables|/Game/MainContent/Blueprints/System/BP_Anomaly.BP_Anomaly_C|GetIsActive _array_element))
                (Development|PrintString (Utilities|String|ToString(Text) (Utilities|Text|FormatText "{CurrentHour}:{CurrentMinute}" (Variables|Default|GetCurrentHour) (Variables|Default|GetCurrentMinute))) true true "(R=0.139990,G=1.000000,B=0.003396,A=1.000000)")
                (Development|PrintString (Utilities|String|ToString(Text) (Utilities|Text|FormatText "{SpawnHour}:{SpawnMinute}" _nextspawnhour _nextspawnminute)) true true "(R=0.118383,G=0.000000,B=1.000000,A=1.000000)")
                (if (and (== _nextspawnminute (Variables|Default|GetCurrentMinute)) (== _nextspawnhour (Variables|Default|GetCurrentHour)))
                  (Development|PrintString "ACTIVATING ANOMALY")
                  (Utilities|Casting|CastToBP_Door_Anomaly_Child _array_element)
                  (Development|PrintString "Door found")
                  (Default|ActivateAnomaly _array_element)
                  (CallFunction|ScheduleNextAnomaly)
                  (Variables|Default|SetbSpawnScheduled true)
                  (goto _label Break)))))))
      (else
        (goto _label)))
    (else
      (goto _label))))

(fn DebugTime
  (Development|PrintString (Utilities|String|Append (Utilities|String|Append (Utilities|String|Append "Time:" (Utilities|String|ToString(Integer) (Variables|Default|GetCurrentHour))) ";") (Utilities|String|ToString(Integer) (Variables|Default|GetCurrentMinute)))))

(fn ScheduleNextAnomaly
  (LocalVariables|SetDelayMinutes (Math|Random|RandomIntegerinRange (Variables|Default|GetMinSpawnDelay) (Variables|Default|GetMaxSpawnDelay)))
  (bind _output_get (Variables|Default|SetNextSpawnHour (Math|Integer|%(Integer) (/ (+ (+ (* (Variables|Default|GetCurrentHour) 60) (Variables|Default|GetCurrentMinute)) (LocalVariables|GetDelayMinutes)) 60) 24)))
  (bind _output_get_2 (Variables|Default|SetNextSpawnMinute (Math|Integer|%(Integer) (+ (+ (* (Variables|Default|GetCurrentHour) 60) (Variables|Default|GetCurrentMinute)) (LocalVariables|GetDelayMinutes)) 60)))
  (LocalVariables|SetDelayMinutes 0)
  (Development|PrintText (Utilities|Text|FormatText "NEXT ANOMALY: {Hour}:{Minute}" _output_get _output_get_2) true true "(R=1.000000,G=0.000000,B=0.930745,A=1.000000)")
  (Variables|Default|SetbSpawnScheduled true))