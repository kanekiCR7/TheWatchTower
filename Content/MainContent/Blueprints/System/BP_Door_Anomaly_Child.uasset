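; Door anomaly child Blueprint that animates a door when the anomaly activates.
; ActivateAnomaly calls the parent, then StartDoorAnimation, which plays a non-looping door animation and sets IsActive.
; A DoOnce with no reset limits this to one play, as ResetAnomaly and DeactivateAnomaly only call the parent.
; BeginPlay caches closed and yaw-offset open rotations, used only by an unconnected leftover timeline that never runs.
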(event Custom|StartDoorAnimation
  (Utilities|FlowControl|DoOnce false
    (:Completed
      (Components|Animation|PlayAnimation (Variables|Default|GetDoor) "/Game/MainContent/Models/Door/wt_door_Anim.wt_door_Anim" false)
      (Variables|Default|SetIsActive true))))

(event EventBeginPlay
  (|CallParentFunction)
  (bind _output_get (Variables|Default|SetClosedRotation (Variables|/Script/Engine.SceneComponent|GetRelativeRotation (Variables|Default|GetDoor))))
  (Variables|Default|SetOpenRotation (Math|Rotator|MakeRotator (.Roll (Math|Rotator|BreakRotator _output_get)) (.Pitch (Math|Rotator|BreakRotator _output_get)) (+ (.Yaw (Math|Rotator|BreakRotator _output_get)) 9e+01))))

(event Collision|EventActorBeginOverlap
  (params (OtherActor :type Actor%20Object%20Reference))
  (|CallParentFunction OtherActor))

(event EventTick
  (params (DeltaSeconds :type Float%20%28single-precision%29))
  (|CallParentFunction DeltaSeconds) ; This node is disabled and will not be called.\nDrag off pins to build functionality.
)

(fn ConstructionScript
  (|CallParentFunction))

(fn ResetAnomaly
  (|CallParentFunction))

(fn DeactivateAnomaly
  (|CallParentFunction))

(fn ActivateAnomaly
  (|CallParentFunction)
  (CallFunction|StartDoorAnimation))